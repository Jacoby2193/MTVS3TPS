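; BP_Player is the third-person shooter player Blueprint, handling HUD, minimap camera and grenade throwing.
; BeginPlay creates the main widget and finds the SceneCapture2D that Tick keeps above the player, while events update the gun UI or show Game Over.
; Pressing G attaches a spawned grenade at GrenadeOrigin, and release launches it with physics force.
; Enhanced Input events are empty; their movement, look, fire and roll logic sits disconnected.
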(event `EnhancedInput|/Game/TPS/Input/Actions/IA_DiveRoll`
  (params (ActionValue :type Boolean) (ElapsedSeconds :type "Float (double-precision)") (TriggeredSeconds :type "Float (double-precision)") (InputAction :type "InputAction Object Reference" :default "/Game/TPS/Input/Actions/IA_DiveRoll.IA_DiveRoll")))

(event `EnhancedInput|/Game/TPS/Input/Actions/IA_Fire`
  (params (ActionValue :type Boolean) (ElapsedSeconds :type "Float (double-precision)") (TriggeredSeconds :type "Float (double-precision)") (InputAction :type "InputAction Object Reference" :default "/Game/TPS/Input/Actions/IA_Fire.IA_Fire")))

(event `self.ShowGameOverUI`
  (bind _returnvalue (`|CreateWidget` "/Game/TPS/UI/WBP_GameOver.WBP_GameOver_C"))
  (`UserWidget.AddToViewport` _returnvalue 0))

(event `self.ChooseSniperGun`
  (params (bSiperGun :type Boolean))
  (bind _mainui (`self.MainUI`)
    (:`then`
      (`/Game/TPS/UI/WBP_Main.ShowGunUI` _mainui bSiperGun))
    (:`else`)))

(event `self.ReceiveBeginPlay`
  (`|ExecutionSequence`
    (:`then_0`
      (bind _returnvalue (`|CreateWidget` "/Game/TPS/UI/WBP_Main.WBP_Main_C"))
      (bind _output_get (set `self.MainUI` _returnvalue))
      (`UserWidget.AddToViewport` _output_get 0)
      (`/Game/TPS/UI/WBP_Main.ShowGunUI` _output_get false))
    (:`then_1`
      (bind _returnvalue_2 (`GameplayStatics.GetActorOfClass` "/Script/Engine.SceneCapture2D"))
      (set `self.MinimapCamera` _returnvalue_2))))

(event `self.ReceiveTick`
  (params (DeltaSeconds :type "Float (single-precision)"))
  (bind (_returnvalue_x _returnvalue_y) (`KismetMathLibrary.BreakVector` (`self.K2_GetActorLocation`)))
  (`self.K2_SetActorLocation` (`self.MinimapCamera`) (`KismetMathLibrary.MakeVector` _returnvalue_x _returnvalue_y 800.0) false false))

(event `EnhancedInput|/Game/TPS/Input/Actions/IA_Move`
  (params (ActionValue :type "Vector2D Structure") (ElapsedSeconds :type "Float (double-precision)") (TriggeredSeconds :type "Float (double-precision)") (InputAction :type "InputAction Object Reference" :default "/Game/TPS/Input/Actions/IA_Move.IA_Move")))

(event `Key|G`
  (params (Key :type "Key Structure"))
  (:`Pressed`
    (bind _returnvalue (`|SpawnActorFromClass` "/Game/TPS/Blueprints/BP_Grenade.BP_Grenade_C" (`SceneComponent.K2_GetComponentToWorld` (`self.GrenadeOrigin`)) "AlwaysSpawn" "MultiplyWithRoot" null null))
    (set `self.GrabGrenade` _returnvalue)
    (`self.K2_AttachToComponent` _returnvalue (`self.GrenadeOrigin`) "None" "SnapToTarget" "SnapToTarget" "KeepRelative" true))
  (:`Released`
    (bind _grabgrenade (`self.GrabGrenade`)
      (:`then`
        (`self.K2_DetachFromActor` _grabgrenade "KeepRelative" "KeepRelative" "KeepRelative")
        (bind _spherecollision (`/Game/TPS/Blueprints/BP_Grenade.SphereCollision` _grabgrenade))
        (`PrimitiveComponent.SetSimulatePhysics` _spherecollision true)
        (set `/Game/TPS/Blueprints/BP_Grenade.bCanOverlap` true _grabgrenade)
        (`PrimitiveComponent.AddForce` _spherecollision (* (`SceneComponent.GetForwardVector` (`self.GrenadeOrigin`)) 100000.0) "None" false)
        (set `self.GrabGrenade` null))
      (:`else`))))

(event `EnhancedInput|/Game/TPS/Input/Actions/IA_Look`
  (params (ActionValue :type "Vector2D Structure") (ElapsedSeconds :type "Float (double-precision)") (TriggeredSeconds :type "Float (double-precision)") (InputAction :type "InputAction Object Reference" :default "/Game/TPS/Input/Actions/IA_Look.IA_Look")))

(fn `UserConstructionScript`)